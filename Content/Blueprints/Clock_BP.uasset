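; Clock actor whose second hand advances on a button's custom tick and raises the player's stress as time runs late.
; BeginPlay sets the SecondBox yaw from the starting second, and Tick re-binds CustomTick to the Trigger Button_BP's dispatcher every frame.
; Each CustomTick rotates the hand one second's step and increments the count; past a threshold, every tick calls MainChar's stress level change dispatcher.
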(event `self.ReceiveBeginPlay`
  (bind _second_box (`self.second_box`))
  (bind (_relativerotation_roll _relativerotation_pitch) (`KismetMathLibrary.BreakRotator` (`SceneComponent.RelativeRotation` _second_box)))
  (`SceneComponent.K2_SetRelativeRotation` _second_box (`KismetMathLibrary.MakeRotator` _relativerotation_roll _relativerotation_pitch (* (`self.current_second`) 6.0)) false false))

(event `self.ReceiveTick`
  (params (DeltaSeconds :type "Float (single-precision)"))
  (bind _asbutton_bp (cast `/Game/Blueprints/Button_BP` (`self.trigger`)))
  (add `/Game/Blueprints/Button_BP.CustomTickDispatcher` _asbutton_bp (delegate `CustomTick`)))

(event `CustomTick`
  (bind _second_box (`self.second_box`))
  (bind (_relativerotation_roll _relativerotation_pitch _relativerotation_yaw) (`KismetMathLibrary.BreakRotator` (`SceneComponent.RelativeRotation` _second_box)))
  (`SceneComponent.K2_SetRelativeRotation` _second_box (`KismetMathLibrary.MakeRotator` _relativerotation_roll _relativerotation_pitch (+ _relativerotation_yaw 6.0)) false false)
  (bind _result (`/Engine/EditorBlueprintResources/StandardMacros.IncrementFloat` (`self.current_second`))
    (:`  `
      (bind _output_get (set `self.current_second` _result))
      (if (> _output_get 50.0)
        (bind _asmain_char (cast `/Game/Blueprints/MainChar` (`GameplayStatics.GetPlayerCharacter` 0)))
        (`/Game/Blueprints/MainChar.StressLevelChangeDispatcher` _asmain_char 10)))))

(fn `UserConstructionScript`)