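; Docs_BP is a clickable document dispenser that hands out a series of texts one at a time.
; On begin play, DocText shows the current entry of the DocsText array.
; Clicking DocBox, while the index is within the array, spawns a Doc_BP slightly above the box carrying the current text.
; It then advances CurrentDoc and updates DocText to preview the next entry.
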(event `self.ReceiveBeginPlay`
  (:`then`
    (`TextRenderComponent.K2_SetText` (`self.DocText`) (`KismetTextLibrary.Conv_StringToText` (`|GetArrayItem` (`self.docs_text`) (`self.current_doc`))))))

(event `self.DocBox.OnClicked`
  (params (TouchedComponent :type "PrimitiveComponent Object Reference") (ButtonPressed :type "Key Structure"))
  (if (< (`self.current_doc`) (`KismetArrayLibrary.Array_Length` (`self.docs_text`)))
    (`|SpawnActorFromClass` "/Game/Blueprints/Doc_BP.Doc_BP_C" (`KismetMathLibrary.MakeTransform` (`KismetMathLibrary.MakeVector` (.x (.location (`SceneComponent.K2_GetComponentToWorld` (`self.DocBox`)))) (.y (.location (`SceneComponent.K2_GetComponentToWorld` (`self.DocBox`)))) (+ (.z (.location (`SceneComponent.K2_GetComponentToWorld` (`self.DocBox`)))) 3.0)) (.rotation (`SceneComponent.K2_GetComponentToWorld` (`self.DocBox`))) (.scale (`SceneComponent.K2_GetComponentToWorld` (`self.DocBox`)))) "Undefined" "OverrideRootScale" null (`|GetArrayItem` (`self.docs_text`) (`self.current_doc`)) null)
    (bind _result (`/Engine/EditorBlueprintResources/StandardMacros.IncrementInt` (`self.current_doc`))
      (:`  `
        (bind _output_get (set `self.current_doc` _result))
        (`TextRenderComponent.K2_SetText` (`self.DocText`) (`KismetTextLibrary.Conv_StringToText` (`|GetArrayItem` (`self.docs_text`) _output_get)))))))

(fn `UserConstructionScript`)