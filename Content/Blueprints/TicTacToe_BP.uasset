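; Tic-tac-toe board actor where the player clicks fields to place O and the computer answers with X in a randomly chosen empty field.
; Marks live in each field mesh's child text component, and grid positions come from numbered component names.
; After each move, IsWinner checks only lines through that cell using modulo wrapping, reveals the matching WinLine component on a win, and further clicks are disabled.
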(event `self.ReceiveBeginPlay`
  (for _array_element (`SceneComponent.GetChildrenComponents` (`self.Fields`) false)
    (bind _astext_render_component (cast `TextRenderComponent` (`SceneComponent.GetChildComponent` _array_element 0)))
    (`TextRenderComponent.K2_SetText` _astext_render_component (`KismetTextLibrary.Conv_StringToText` ""))
    (for _array_element_2 (`SceneComponent.GetChildrenComponents` (`self.WinLines`) false)
      (`SceneComponent.SetVisibility` _array_element_2 false false))
    (for _array_element_3 (`SceneComponent.GetChildrenComponents` (`self.Fields`) false)
      (bind _asstatic_mesh_component (cast `StaticMeshComponent` _array_element_3))
      (add `PrimitiveComponent.OnClicked` _asstatic_mesh_component (delegate `OnClicked_Event_1`)))))

(event `OnClicked_Event_1`
  (params (TouchedComponent :type "PrimitiveComponent Object Reference") (ButtonPressed :type "Key Structure" :default "None"))
  (bind _fields (`self.Fields`))
  (bind _returnvalue (`SceneComponent.GetChildComponent` _fields (`self.emptyFieldIndex`)))
  (if (not (`self.disabled`))
    (bind _astext_render_component (cast `TextRenderComponent` (`SceneComponent.GetChildComponent` TouchedComponent 0)))
    (if (`KismetTextLibrary.TextIsEmpty` (`TextRenderComponent.Text` _astext_render_component))
      (`TextRenderComponent.K2_SetText` _astext_render_component (`KismetTextLibrary.Conv_StringToText` "O"))
      (bind _winning (`self.IsWinner` "O" (- (`KismetStringLibrary.Conv_StringToInt` (`KismetStringLibrary.Replace` (`KismetSystemLibrary.GetObjectName` TouchedComponent) "Field")) 1)))
      (if _winning
        (set `self.disabled` true)
        (else
          (bind _emptyexist (`self.IsThereEmptyField`))
          (bind _output_get (set `self.isCellFilled` _emptyexist))
          (while _output_get
            (bind _output_get_2 (set `self.emptyFieldIndex` (`KismetMathLibrary.RandomIntegerInRange` 0 (`SceneComponent.GetNumChildrenComponents` _fields))))
            (bind _astext_render_component_2 (cast `TextRenderComponent` (`SceneComponent.GetChildComponent` (`SceneComponent.GetChildComponent` _fields _output_get_2) 0)))
            (set `self.isCellFilled` (not (`KismetTextLibrary.TextIsEmpty` (`TextRenderComponent.Text` _astext_render_component_2)))))
          (bind _astext_render_component_3 (cast `TextRenderComponent` (`SceneComponent.GetChildComponent` _returnvalue 0)))
          (`TextRenderComponent.K2_SetText` _astext_render_component_3 (`KismetTextLibrary.Conv_StringToText` "X"))
          (bind _winning_2 (`self.IsWinner` "X" (- (`KismetStringLibrary.Conv_StringToInt` (`KismetStringLibrary.Replace` (`KismetSystemLibrary.GetObjectName` _returnvalue) "Field")) 1)))
          (if _winning_2
            (set `self.disabled` true)))))))

(fn `FindComponentByIndex`
  (params (components :type "Array of SceneComponent Object Reference") (prefix :type String) (index :type Integer))
  (returns (result :type "SceneComponent Object Reference"))
  (for _array_element components
    (if (`KismetStringLibrary.EqualEqual_StrStr` (`KismetSystemLibrary.GetObjectName` _array_element) (`KismetStringLibrary.Concat_StrStr` prefix (`KismetStringLibrary.Conv_IntToString` (+ index 1))))
      (break)))
  (return _array_element))

(fn `GetFieldValue`
  (params (x :type Integer) (y :type Integer))
  (returns (FieldValue :type String))
  (for _array_element (`SceneComponent.GetChildrenComponents` (`self.Fields`) false)
    (if (`KismetStringLibrary.EqualEqual_StrStr` (`KismetSystemLibrary.GetObjectName` _array_element) (`KismetStringLibrary.Concat_StrStr` "Field" (`KismetStringLibrary.Conv_IntToString` (+ x (* y 3) 1))))
      (break)))
  (bind _astext_render_component (cast `TextRenderComponent` (`SceneComponent.GetChildComponent` _array_element 0)))
  (return (`KismetTextLibrary.Conv_TextToString` (`TextRenderComponent.Text` _astext_render_component))))

(fn `IsThereEmptyField`
  (returns (EmptyExist :type Boolean))
  (locals (IsEmptyFields :type Boolean))
  (for _array_element (`SceneComponent.GetChildrenComponents` (`self.Fields`) false)
    (bind _astext_render_component (cast `TextRenderComponent` (`SceneComponent.GetChildComponent` _array_element 0)))
    (set `local.IsEmptyFields` (or (`KismetTextLibrary.TextIsEmpty` (`TextRenderComponent.Text` _astext_render_component)) (`local.IsEmptyFields`))))
  (return (`local.IsEmptyFields`)))

(fn `IsWinner`
  (params (player :type String) (IndexCheck :type Integer))
  (returns (winning :type Boolean))
  (locals (x :type Integer) (y :type Integer) (IsDiagonal1Win :type Boolean :default true) (IsHorizontalWin :type Boolean :default true) (IsVerticalWin :type Boolean :default true) (IsDiagonal2Win :type Boolean :default true))
  (bind _isdiagonal1win (`local.IsDiagonal1Win`))
  (bind _ishorizontalwin (`local.IsHorizontalWin`))
  (bind _isverticalwin (`local.IsVerticalWin`))
  (bind _isdiagonal2win (`local.IsDiagonal2Win`))
  (bind _x (`local.x`))
  (bind _y (`local.y`))
  (set `local.y` (/ IndexCheck 3))
  (set `local.x` (mod IndexCheck 3))
  (for _index (range 3)
    (bind _fieldvalue (`self.GetFieldValue` (mod (+ _index (`local.x`)) 3) (`local.y`)))
    (if (not (`KismetStringLibrary.EqualEqual_StrStr` _fieldvalue player))
      (set `local.IsHorizontalWin` false))
    (bind _fieldvalue_2 (`self.GetFieldValue` (`local.x`) (mod (+ _index (`local.y`)) 3)))
    (if (not (`KismetStringLibrary.EqualEqual_StrStr` _fieldvalue_2 player))
      (set `local.IsVerticalWin` false))
    (if (== _x _y)
      (bind _fieldvalue_3 (`self.GetFieldValue` (mod (+ _index (`local.x`)) 3) (mod (+ _index (`local.y`)) 3)))
      (if (not (`KismetStringLibrary.EqualEqual_StrStr` _fieldvalue_3 player))
        (set `local.IsDiagonal1Win` false))
      (if (and (== (`local.y`) 1) (== (`local.x`) 1))
        (bind _fieldvalue_4 (`self.GetFieldValue` (mod (+ _index (`local.x`)) 3) (mod (+ (* _index 2) (`local.y`)) 3) :!label _label))
        (if (not (`KismetStringLibrary.EqualEqual_StrStr` _fieldvalue_4 player))
          (set `local.IsDiagonal2Win` false)
          (set `local.IsDiagonal1Win` false))
        (else
          (set `local.IsDiagonal2Win` false)))
      (else
        (set `local.IsDiagonal1Win` false)
        (if (or (and (== _x 0) (== _y 2)) (and (== _y 0) (== _x 2)) false)
          (goto _label)
          (else
            (set `local.IsDiagonal2Win` false))))))
  (if _isdiagonal1win
    (`SceneComponent.SetVisibility` (`self.WinLine8`) true false)
    (elif _ishorizontalwin
      (bind _result (`self.FindComponentByIndex` (`SceneComponent.GetChildrenComponents` (`self.WinLines`) false) "WinLine" (+ (`local.y`) 3)))
      (`SceneComponent.SetVisibility` _result true false)
      (elif _isverticalwin
        (bind _result_2 (`self.FindComponentByIndex` (`SceneComponent.GetChildrenComponents` (`self.WinLines`) false) "WinLine" (`local.x`)))
        (`SceneComponent.SetVisibility` _result_2 true false)
        (elif _isdiagonal2win
          (`SceneComponent.SetVisibility` (`self.WinLine7`) true false)))))
  (return (or _isdiagonal1win _ishorizontalwin _isverticalwin _isdiagonal2win)))

(fn `UserConstructionScript`)