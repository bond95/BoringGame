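; MainChar is the player character Blueprint, providing mouse look, centre-screen click interaction and an initial stress readout.
; Look axis inputs drive controller yaw and pitch, while Tick pins the mouse cursor to the viewport centre every frame.
; BeginPlay enables click events, adds a CenterDot widget, then writes the Stress value once into the Level text of the Stress_BP monitor.
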(event `self.ReceiveTick`
  (params (DeltaSeconds :type "Float (single-precision)"))
  (bind (_returnvalue_x _returnvalue_y) (`KismetMathLibrary.BreakVector2D` (`WidgetLayoutLibrary.GetViewportSize`)))
  (`PlayerController.SetMouseLocation` (`GameplayStatics.GetPlayerController` 0) (`KismetMathLibrary.FTrunc` (/ _returnvalue_x 2.0)) (`KismetMathLibrary.FTrunc` (/ _returnvalue_y 2.0))))

(event `self.ReceiveBeginPlay`
  (set `PlayerController.bEnableClickEvents` true (`GameplayStatics.GetPlayerController` 0))
  (bind _returnvalue (`|CreateWidget` "/Game/Blueprints/CenterDot.CenterDot_C"))
  (`UserWidget.AddToViewport` _returnvalue 0)
  (bind _asstress_bp (cast `/Game/Blueprints/Stress_BP` (`self.stress_monitor`)))
  (`TextRenderComponent.K2_SetText` (`/Game/Blueprints/Stress_BP.level` _asstress_bp) (`KismetTextLibrary.Conv_IntToText` (`self.stress`))))

(event `InputAxis|Look_turn`
  (params (AxisValue :type "Float (single-precision)"))
  (`self.AddControllerYawInput` AxisValue))

(event `InputAxis|Look_up`
  (params (AxisValue :type "Float (single-precision)"))
  (`self.AddControllerPitchInput` AxisValue))

(fn `UserConstructionScript`)