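; Document actor that shows configurable text and lets the player click to sign it or decline.
; BeginPlay fills the document text from a variable.
; Clicking either sign component writes the signed text and plays the end sequence, while either decline component plays the same sequence without signing.
; When the EndSequence component deactivates, the root scene component is destroyed.
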(event `self.ReceiveBeginPlay`
  (`TextRenderComponent.K2_SetText` (`self.DocText`) (`KismetTextLibrary.Conv_StringToText` (`self.Text`))))

(event `self.SignBox.OnClicked`
  (params (TouchedComponent :type "PrimitiveComponent Object Reference") (ButtonPressed :type "Key Structure"))
  (`TextRenderComponent.K2_SetText` (`self.SignText`) (`self.Signed`) :!label _label)
  (`MovieSceneSequencePlayer.Play` (`ActorSequenceComponent.SequencePlayer` (`self.EndSequence`)) :!label _label_2))

(event `self.SignAction.OnClicked`
  (params (TouchedComponent :type "PrimitiveComponent Object Reference") (ButtonPressed :type "Key Structure"))
  (goto _label))

(event `self.NotSignBox.OnClicked`
  (params (TouchedComponent :type "PrimitiveComponent Object Reference") (ButtonPressed :type "Key Structure"))
  (goto _label_2))

(event `self.NotSign.OnClicked`
  (params (TouchedComponent :type "PrimitiveComponent Object Reference") (ButtonPressed :type "Key Structure"))
  (goto _label_2))

(event `self.EndSequence.OnComponentDeactivated`
  (params (Component :type "ActorComponent Object Reference"))
  (`ActorComponent.K2_DestroyComponent` (`self.DefaultSceneRoot`)))

(fn `UserConstructionScript`)