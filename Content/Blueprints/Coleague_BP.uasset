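; Colleague actor that performs a random idle activity while the player looks toward it, and passes that activity to the player on click.
; Tick runs a dot-product view-cone check against control rotation, without testing occlusion.
; Entering view starts either smoking with a hand-socketed cigarette or a looping RoundSequence; leaving view stops and resets it.
; Clicking the box or mesh calls the matching SetSmoking or SetRolling on MainChar.
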(event `self.ReceiveTick`
  (params (DeltaSeconds :type "Float (single-precision)"))
  (bind _cigarete (`self.Cigarete`))
  (bind _cigarete_2 (`self.Cigarete`))
  (bind _isobservable (`self.IsObservable`))
  (if (!= _isobservable (`self.InViewport`))
    (bind _output_get (set `self.InViewport` _isobservable))
    (if _output_get
      (bind _output_get_2 (set `self.CurrentAnimation` (`KismetMathLibrary.RandomInteger` 2)))
      (switch `int` _output_get_2
        (:`0`
          (`SceneComponent.K2_AttachToComponent` _cigarete_2 (`self.SkeletalMesh`) "hand_rSocket" "KeepRelative" "KeepRelative" "KeepRelative" true)
          (`SceneComponent.SetVisibility` _cigarete_2 true false)
          (`self.SmokeDispatch`))
        (:`1`
          (`MovieSceneSequencePlayer.PlayLooping` (`ActorSequenceComponent.SequencePlayer` (`self.RoundSequence`)) -1)))
      (else
        (switch `int` (`self.CurrentAnimation`)
          (:`0`
            (`SceneComponent.K2_DetachFromComponent` _cigarete "KeepRelative" "KeepRelative" "KeepRelative" true)
            (`SceneComponent.SetVisibility` _cigarete false false)
            (`self.InitDispatch`))
          (:`1`
            (`MovieSceneSequencePlayer.GoToEndAndStop` (`ActorSequenceComponent.SequencePlayer` (`self.RoundSequence`)))))
        (set `self.CurrentAnimation` -1)))))

(event `self.Box.OnClicked`
  (params (TouchedComponent :type "PrimitiveComponent Object Reference") (ButtonPressed :type "Key Structure"))
  (bind _asmain_char (cast `/Game/Blueprints/MainChar` (`GameplayStatics.GetPlayerCharacter` 0) :!label _label))
  (switch `int` (`self.CurrentAnimation`)
    (:`0`
      (`/Game/Blueprints/MainChar.SetSmoking` _asmain_char))
    (:`1`
      (`/Game/Blueprints/MainChar.SetRolling` _asmain_char))))

(event `self.SkeletalMesh.OnClicked`
  (params (TouchedComponent :type "PrimitiveComponent Object Reference") (ButtonPressed :type "Key Structure"))
  (goto _label))

(fn `IsObservable`
  (returns (IsObservable :type Boolean))
  (return (>= (* (`KismetMathLibrary.Dot_VectorVector` (`KismetMathLibrary.GetForwardVector` (`KismetMathLibrary.FindLookAtRotation` (`self.K2_GetActorLocation`) (`self.K2_GetActorLocation` (`GameplayStatics.GetPlayerPawn` 0)))) (`KismetMathLibrary.GetForwardVector` (`Controller.GetControlRotation` (`GameplayStatics.GetPlayerController` 0)))) -1.0) 0.7)))

(fn `UserConstructionScript`)