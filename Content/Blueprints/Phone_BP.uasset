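; Clickable phone actor that toggles between picking up and putting down the phone through a Level Sequence.
; Clicking with the headset visible plays the pickup sequence if idle, and its forward finish hides the headset.
; Clicking with the headset hidden plays the sequence in reverse and immediately shows the headset again.
; The finish callback is reassigned on every Tick rather than once at BeginPlay.
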(event `self.Phone.OnClicked`
  (params (TouchedComponent :type "PrimitiveComponent Object Reference") (ButtonPressed :type "Key Structure"))
  (bind _returnvalue (`SceneComponent.IsVisible` (`self.Headset`)))
  (bind _sequenceplayer (`ActorSequenceComponent.SequencePlayer` (`self.PickupPhoneSequence`)))
  (if (and _returnvalue (not (`MovieSceneSequencePlayer.IsPlaying` _sequenceplayer)))
    (`MovieSceneSequencePlayer.Play` _sequenceplayer)
    (elif (not _returnvalue)
      (`MovieSceneSequencePlayer.PlayReverse` _sequenceplayer)
      (`SceneComponent.SetVisibility` (`self.Headset`) true false))))

(event `self.ReceiveTick`
  (params (DeltaSeconds :type "Float (single-precision)"))
  (add `MovieSceneSequencePlayer.OnFinished` (`ActorSequenceComponent.SequencePlayer` (`self.PickupPhoneSequence`)) (delegate `OnFinished_Event_0`)))

(event `OnFinished_Event_0`
  (if (not (`MovieSceneSequencePlayer.IsReversed` (`ActorSequenceComponent.SequencePlayer` (`self.PickupPhoneSequence`))))
    (`SceneComponent.SetVisibility` (`self.Headset`) false false)))

(fn `UserConstructionScript`)